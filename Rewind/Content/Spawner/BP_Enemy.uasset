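; Enemy for a rhythm-themed game that chases the RewindChracter player with AIMoveTo, starting 1.2 seconds after spawn.
; A Ritmo event flashes its point light in a given color, and player overlap brightens it.
; Bullet overlap explodes it and adds score to RewindGM, doubled during the spawn delay.
; Bullet hits stop movement and drive a timeline effect on a dynamic material from the impacting bullet's position.
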(event OnComponentBeginOverlap(CapsuleComponent)
  (params (OverlappedComponent :type Primitive%20Component%20Object%20Reference) (OtherActor :type Actor%20Object%20Reference) (OtherComp :type Primitive%20Component%20Object%20Reference) (OtherBodyIndex :type Integer) (bFromSweep :type Boolean) (SweepResult :type Hit%20Result%20Structure%20%28by%20ref%29))
  (Utilities|FlowControl|Sequence
    (:then_0
      (Utilities|Casting|CastToRewindChracter OtherActor)
      (bind _output_get (Variables|Default|SetIsInRadious true))
      (Rendering|Components|Light|SetIntensity (Variables|Default|GetPointLight) 2e+05))
    (:then_1
      ;[1 1 1] interaction
      (bind _asbp_bullet (Utilities|Casting|CastToBP_Bullet OtherActor))
      (Variables|Default|SetDead true)
      (Components|Movement|StopMovementImmediately (Variables|Character|GetCharacterMovement))
      (Effects|SpawnEmitteratLocation "/Game/Explosion/Explosion/P_Explosion.P_Explosion" (Transformation|GetWorldLocation (Variables|Character|GetMesh)))
      (Actor|DestroyActor)
      (bind _asrewind_gm (Utilities|Casting|CastToRewindGM (Game|GetGameMode)))
      (if (Variables|Default|GetIsInTime)
        (Variables|/Game/Blueprints/RewindGM.RewindGM_C|SetScore _asrewind_gm (+ (Variables|/Game/Blueprints/RewindGM.RewindGM_C|GetScore _asrewind_gm) 2))
        (else
          (Variables|/Game/Blueprints/RewindGM.RewindGM_C|SetScore _asrewind_gm (+ (Variables|/Game/Blueprints/RewindGM.RewindGM_C|GetScore _asrewind_gm) 1))))
      (Actor|DestroyActor _asbp_bullet)
      (Audio|PlaySoundatLocation "/Game/Audio/Beat.Beat" "0, 0, 0" "0, 0, 0" 1.0 1.0 0.0 0 0 0))))

(event OnComponentHit(CapsuleComponent)
  (params (HitComponent :type Primitive%20Component%20Object%20Reference) (OtherActor :type Actor%20Object%20Reference) (OtherComp :type Primitive%20Component%20Object%20Reference) (NormalImpulse :type Vector :default "0, 0, 0") (Hit :type Hit%20Result%20Structure%20%28by%20ref%29))
  (bind _material (Variables|Default|GetMaterial))
  (bind _asbp_bullet (Utilities|Casting|CastToBP_Bullet OtherActor))
  (Development|PrintString "success")
  (Components|Movement|StopMovementImmediately (Variables|Character|GetCharacterMovement))
  (Rendering|Material|SetVectorParameterValue _material "Location" (Math|Conversions|ToLinearColor(Vector) (Transformation|GetWorldLocation (Variables|/Game/ThirdPersonCPP/Blueprints/ThirdPersonBP/Blueprints/BP_Bullet.BP_Bullet_C|GetSphere _asbp_bullet))) :!class /Script/Engine.MaterialInstanceDynamic)
  (bind _effect (Timeline|Timeline_0 Play)
    (:Update
      (Rendering|Material|SetScalarParameterValue _material "Amount" _effect :!class /Script/Engine.MaterialInstanceDynamic)
      (Development|PrintString "get hit"))))

(event Custom|Ritmo
  (params (Color :type Float%20%28single-precision%29) (Color1 :type Float%20%28single-precision%29) (Color2 :type Float%20%28single-precision%29) (Percussion :type Time%20Synth%20Component%20Object%20Reference))
  (bind _pointlight (Variables|Default|GetPointLight))
  ;[1 1 1] light
  (Rendering|SetVisibility _pointlight true false)
  (Rendering|Components|Light|SetLightColor (Variables|Default|GetPointLight) (Math|Color|MakeColor Color Color1 Color2) true)
  (Variables|Default|SetIsPlayingtheBeat true)
  (if (Variables|Default|GetIsInRadious)
    (Utilities|FlowControl|Delay 1.2)
    (else
      (Utilities|FlowControl|Delay (Variables|Default|GetLightTime))))
  (Rendering|SetVisibility _pointlight false false)
  (Variables|Default|SetIsPlayingtheBeat false))

(event EventBeginPlay
  (Variables|Default|SetIsInTime true)
  (Utilities|FlowControl|Sequence
    (:then_0
      (Utilities|FlowControl|Delay 1.2)
      ;[1 1 1] followPlayer
      (bind _asrewind_chracter (Utilities|Casting|CastToRewindChracter (Game|Player|GetPlayerPawn 0)))
      (bind _output_get (Variables|Default|SetChracter _asrewind_chracter))
      (Utilities|IsValid _output_get
        (:Is%20Valid
          (Variables|Default|SetIsInTime false)
          (if (not (Variables|Default|GetDead))
            (AI|AIMoveTo self (Transformation|GetWorldLocation (Variables|/Script/Engine.Character|GetMesh (Variables|Default|GetChracter))) (Variables|Default|GetChracter) 5.0 false)))))
    (:then_1
      (Rendering|SetVisibility (Variables|Default|GetPointLight) false false))
    (:then_3
      (bind _returnvalue (Rendering|Material|CreateDynamicMaterialInstance (Variables|Character|GetMesh) 0 0 "None" :!class /Script/Engine.PrimitiveComponent))
      (Variables|Default|SetMaterial _returnvalue))))

(event EventTick
  (params (DeltaSeconds :type Float%20%28single-precision%29))
  (bind _chracter (Variables|Default|GetChracter))
  ;[1 1 1] followPlayer
  (Utilities|IsValid _chracter
    (:Is%20Valid
      (if (not (Variables|Default|GetDead))
        (AI|AIMoveTo self (Transformation|GetWorldLocation (Variables|/Script/Engine.Character|GetMesh _chracter)) _chracter 5.0 false)))))

(fn ConstructionScript)