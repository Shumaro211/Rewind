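; BP_Spawner is a music-driven enemy spawner that plays a layered song and turns its beats into gameplay.
; Playing starts or stops three TimeSynth stems (instrumental, kick, percussion) and clears existing enemies.
; Spectral peaks, gated by delay cooldowns, make kick spawn BP_Enemy AI near one of four arrows and percussion call Ritmo on all enemies with random colors.
; Tick re-attaches the spawner to the Character every frame.
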(event Custom|CustomEvent
  (params (SynthPlaybackTimeSeconds :type Float%20%28single-precision%29))
  ;[1 1 1] SongSpawner
  (for _array_element (Class|TimeSynthComponent|GetSpectralData (Variables|Default|GetTimeSynthMasterInstrumental))
    (if (and (> (.Magnitude (Utilities|Struct|BreakTimeSynthSpectralData _array_element)) 91.0) true)
      _)))

(event Custom|SpawnEnemy
  ;[1 1 1] Spawner
  (switch int (Math|Random|RandomIntegerinRange 0 3)
    (:0
      (bind _randomlocation (Class|NavigationSystemV1|GetRandomLocationinNavigableRadius (Transformation|GetWorldLocation (Variables|Default|GetArrow)) 1e+02 0 0))
      (bind _returnvalue (AI|SpawnAIFromClass "/Game/Spawner/BP_Enemy.BP_Enemy_C" "/Game/Spawner/Enemy/BT_Enemy.BT_Enemy" (+ _randomlocation "0, 0,100.000000") "0, 0, 0" true 0))
      (bind _asbp_enemy (Utilities|Casting|CastToBP_Enemy _returnvalue))
      (Variables|/Game/Spawner/BP_Enemy.BP_Enemy_C|SetSpawner _asbp_enemy self))
    (:1
      (bind _randomlocation_2 (Class|NavigationSystemV1|GetRandomLocationinNavigableRadius (Transformation|GetWorldLocation (Variables|Default|GetArrow1)) 1e+02 0 0))
      (bind _returnvalue_2 (AI|SpawnAIFromClass "/Game/Spawner/BP_Enemy.BP_Enemy_C" "/Game/Spawner/Enemy/BT_Enemy.BT_Enemy" (+ _randomlocation_2 "0, 0,100.000000") "0, 0, 0" true 0))
      (bind _asbp_enemy_2 (Utilities|Casting|CastToBP_Enemy _returnvalue_2))
      (Variables|/Game/Spawner/BP_Enemy.BP_Enemy_C|SetSpawner _asbp_enemy_2 self))
    (:2
      (bind _randomlocation_3 (Class|NavigationSystemV1|GetRandomLocationinNavigableRadius (Transformation|GetWorldLocation (Variables|Default|GetArrow2)) 1e+02 0 0))
      (bind _returnvalue_3 (AI|SpawnAIFromClass "/Game/Spawner/BP_Enemy.BP_Enemy_C" "/Game/Spawner/Enemy/BT_Enemy.BT_Enemy" (+ _randomlocation_3 "0, 0,100.000000") "0, 0, 0" true 0))
      (bind _asbp_enemy_3 (Utilities|Casting|CastToBP_Enemy _returnvalue_3))
      (Variables|/Game/Spawner/BP_Enemy.BP_Enemy_C|SetSpawner _asbp_enemy_3 self))
    (:3
      (bind _randomlocation_4 (Class|NavigationSystemV1|GetRandomLocationinNavigableRadius (Transformation|GetWorldLocation (Variables|Default|GetArrow3)) 1e+02 0 0))
      (bind _returnvalue_4 (AI|SpawnAIFromClass "/Game/Spawner/BP_Enemy.BP_Enemy_C" "/Game/Spawner/Enemy/BT_Enemy.BT_Enemy" (+ _randomlocation_4 "0, 0,100.000000") "0, 0, 0" true 0))
      (bind _asbp_enemy_4 (Utilities|Casting|CastToBP_Enemy _returnvalue_4))
      (Variables|/Game/Spawner/BP_Enemy.BP_Enemy_C|SetSpawner _asbp_enemy_4 self))))

(event Custom|PlayPercussion
  (params (SynthPlaybackTimeSeconds :type Float%20%28single-precision%29))
  (bind _timesynthpercussion (Variables|Default|GetTimeSynthPercussion))
  ;[1 1 1] LightSpawner
  (if (Variables|Default|GetIsPlaying)
    (for _array_element (Class|TimeSynthComponent|GetSpectralData (Variables|Default|GetTimeSynthPercussion))
      (if (and (> (.Magnitude (Utilities|Struct|BreakTimeSynthSpectralData _array_element)) 4e+01) (Variables|Default|GetTiempoBitPercussion))
        (Variables|Default|SetTiempoBitPercussion false)
        (Utilities|FlowControl|Delay (Variables|Default|GetTiempobetweenPercussion))
        (Variables|Default|SetTiempoBitPercussion true)
        (bind _outactors (Actor|GetAllActorsOfClass "/Game/Spawner/BP_Enemy.BP_Enemy_C"))
        (for _array_element_2 _outactors
          (switch int (Math|Random|RandomIntegerinRange 0 1)
            (:0
              (Default|Ritmo _array_element_2 255.0 0.0 255.0 _timesynthpercussion))
            (:1
              (Default|Ritmo _array_element_2 255.0 255.0 0.0 _timesynthpercussion))))))))

(event Custom|Playing
  (params (Character :type Rewind%20Chracter%20Object%20Reference))
  (bind _frecuencias (Variables|Default|GetFrecuencias))
  (bind _tiempobetweengobalbpm (Variables|Default|GetTiempobetweenGobalBPM))
  ;[1 1 1] play the game
  (bind _outactors (Actor|GetAllActorsOfClass "/Game/Spawner/BP_Enemy.BP_Enemy_C"))
  (Actor|DestroyActor _outactors)
  (if (Variables|Default|GetIsPlaying)
    ;[1 1 1] LightSpawner
    (Variables|Default|SetTiempoBitPercussion true)
    (Variables|Default|SetTiempoBitKick true)
    (Utilities|FlowControl|Sequence
      (:then_0
        (bind _returnvalue (AddComponent|AddTimeSynthComponent false))
        (Variables|Default|SetTimeSynthMasterInstrumental _returnvalue))
      (:then_1
        (bind _returnvalue_2 (AddComponent|AddTimeSynthComponent false))
        (bind _output_get (Variables|Default|SetTimeSynthKick _returnvalue_2))
        (Variables|/Script/TimeSynth.TimeSynthComponent|SetbEnableSpectralAnalysis _output_get true))
      (:then_2
        (bind _returnvalue_3 (AddComponent|AddTimeSynthComponent false))
        (bind _output_get_2 (Variables|Default|SetTimeSynthPercussion _returnvalue_3))
        (Variables|/Script/TimeSynth.TimeSynthComponent|SetbEnableSpectralAnalysis _output_get_2 true)
        (for _index (range 0 9)
          (Utilities|Array|Add _frecuencias (* _index 5e+01)))
        (Variables|/Script/TimeSynth.TimeSynthComponent|SetFrequenciesToAnalyze (Variables|Default|GetTimeSynthKick) _frecuencias)
        (Variables|/Script/TimeSynth.TimeSynthComponent|SetFrequenciesToAnalyze (Variables|Default|GetTimeSynthPercussion) _frecuencias)
        (Class|TimeSynthComponent|SetBPM (Variables|Default|GetTimeSynthMasterInstrumental) _tiempobetweengobalbpm)
        (Class|TimeSynthComponent|SetBPM (Variables|Default|GetTimeSynthKick) _tiempobetweengobalbpm)
        (Class|TimeSynthComponent|SetBPM (Variables|Default|GetTimeSynthPercussion) _tiempobetweengobalbpm)
        (Utilities|FlowControl|Sequence
          (:then_0
            _)
          (:then_1
            (Utilities|FlowControl|Delay 0.3)
            (Audio|Components|Audio|SetVolumeMultiplier (Variables|Default|GetTimeSynthMasterInstrumental) 1.0 :!class /Script/AudioMixer.SynthComponent)
            (bind _returnvalue_4 (Class|TimeSynthComponent|PlayClip (Variables|Default|GetTimeSynthMasterInstrumental) "/Game/Audio/INSTRUMENTAL_CLI.INSTRUMENTAL_CLI" "/Game/Audio/VolumeSilence.VolumeSilence"))))
        (Audio|Components|Audio|SetVolumeMultiplier (Variables|Default|GetTimeSynthKick) (Variables|Default|GetVolumeKick) :!class /Script/AudioMixer.SynthComponent)
        (bind _returnvalue_5 (Class|TimeSynthComponent|PlayClip (Variables|Default|GetTimeSynthKick) "/Game/Audio/KICK_CLI.KICK_CLI" "/Game/Audio/VolumeSilence.VolumeSilence"))
        (EventDispatchers|BindEventtoOnPlaybackTime (Variables|Default|GetTimeSynthKick) (delegate Custom|Kick%20Play))
        (Audio|Components|Audio|SetVolumeMultiplier (Variables|Default|GetTimeSynthPercussion) (Variables|Default|GetVolumePercussion) :!class /Script/AudioMixer.SynthComponent)
        (bind _returnvalue_6 (Class|TimeSynthComponent|PlayClip (Variables|Default|GetTimeSynthPercussion) "/Game/Audio/PERCUSSION_Cli.PERCUSSION_Cli" "/Game/Audio/VolumeSilence.VolumeSilence"))
        (EventDispatchers|BindEventtoOnPlaybackTime (Variables|Default|GetTimeSynthPercussion) (delegate Custom|PlayPercussion))))
    (else
      (Audio|Components|Audio|Stop (Variables|Default|GetTimeSynthMasterInstrumental))
      (Class|TimeSynthComponent|StopClip (Variables|Default|GetTimeSynthMasterInstrumental) _returnvalue_4 "Global")
      (Audio|Components|Audio|Stop (Variables|Default|GetTimeSynthPercussion))
      (Class|TimeSynthComponent|StopClip (Variables|Default|GetTimeSynthPercussion) _returnvalue_6 "Global")
      (Audio|Components|Audio|Stop (Variables|Default|GetTimeSynthKick))
      (Class|TimeSynthComponent|StopClip (Variables|Default|GetTimeSynthKick) _returnvalue_5 "Global")
      (bind _outactors_2 (Actor|GetAllActorsOfClass "/Game/Spawner/BP_Enemy.BP_Enemy_C"))
      (Actor|DestroyActor _outactors_2))))

(event Custom|Kick%20Play
  (params (SynthPlaybackTimeSeconds :type Float%20%28single-precision%29))
  ;[1 1 1] Kick
  (if (Variables|Default|GetIsPlaying)
    (for _array_element (Class|TimeSynthComponent|GetSpectralData (Variables|Default|GetTimeSynthKick))
      (if (and (> (.Magnitude (Utilities|Struct|BreakTimeSynthSpectralData _array_element)) 1.5) (Variables|Default|GetTiempoBitKick))
        (Variables|Default|SetTiempoBitKick false)
        (Utilities|FlowControl|Delay (Variables|Default|GetTiempobetweenKick))
        (Variables|Default|SetTiempoBitKick true)
        (CallFunction|SpawnEnemy)))))

(event EventTick
  (params (DeltaSeconds :type Float%20%28single-precision%29))
  ;[1 1 1] attach
  (Transformation|AttachActorToActor (stale Custom|Playing Character) "None" "KeepWorld" "KeepWorld" "KeepWorld" true))

(fn ConstructionScript)