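; Actor that shows game-over and menu overlay planes based on the state of the RewindGM game mode.
; Both planes start hidden on BeginPlay.
; Every Tick it casts the game mode to RewindGM and shows Plane while IsDead is set and Plane1 while IsOnMenu is set, hiding each otherwise.
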(event EventBeginPlay
  (Rendering|SetVisibility (Variables|Default|GetPlane) false false)
  (Rendering|SetVisibility (Variables|Default|GetPlane1) false false))

(event EventTick
  (params (DeltaSeconds :type Float%20%28single-precision%29))
  (bind _plane (Variables|Default|GetPlane))
  (bind _plane1 (Variables|Default|GetPlane1))
  (bind _asrewind_gm (Utilities|Casting|CastToRewindGM (Game|GetGameMode)))
  (Utilities|FlowControl|Sequence
    (:then_0
      (if (Variables|/Game/Blueprints/RewindGM.RewindGM_C|GetIsDead _asrewind_gm)
        (Rendering|SetVisibility _plane true false)
        (else
          (Rendering|SetVisibility _plane false false))))
    (:then_1
      (if (Variables|/Game/Blueprints/RewindGM.RewindGM_C|GetIsOnMenu _asrewind_gm)
        (Rendering|SetVisibility _plane1 true false)
        (else
          (Rendering|SetVisibility _plane1 false false))))))

(fn ConstructionScript)